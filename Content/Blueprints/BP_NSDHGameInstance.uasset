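; Game instance for NoSunDownHear that opens the game world level and manages persistent global options.
; GetGlobalOptions loads the options from the GlobalOptions save slot, creating it with defaults if missing.
; SetGlobalOptions applies music and SFX toggles as sound class overrides on SM_Mixer, then overwrites that slot with a new save object.
; The Instant flag controls only the SFX fade, while the music fade follows the SFX toggle.
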(event `LoadGameLevel`
  (`WidgetLayoutLibrary.RemoveAllWidgets`)
  (`GameplayStatics.OpenLevel` "NoSunDownHear_World" false))

(fn `GetGlobalOptions`
  (returns (GlobalOptions :type "/Game/Blueprints/SaveGame/GlobalOptionsStruct Structure"))
  ;[1 1 1] 'GlobalOptions' 이름으로 저장된 옵션이 있는지 확인
  (bind _returnvalue (`GameplayStatics.DoesSaveGameExist` "GlobalOptions"))
  (if _returnvalue
    ;[1 1 1] 있다면 로드 후 구조체 값 반환
    (bind _returnvalue_2 (`GameplayStatics.LoadGameFromSlot` "GlobalOptions"))
    (bind _asglobal_options_save_game (cast `/Game/Blueprints/SaveGame/GlobalOptionsSaveGame` _returnvalue_2))
    (return (`/Game/Blueprints/SaveGame/GlobalOptionsSaveGame.GlobalOptions` _asglobal_options_save_game))
    (else
      ;[1 1 1] 없다면 'GlobalOptions' 이름으로 슬롯 생성 후 구조체 값 반환
      (bind _returnvalue_3 (`GameplayStatics.CreateSaveGameObject` "/Game/Blueprints/SaveGame/GlobalOptionsSaveGame.GlobalOptionsSaveGame_C"))
      (`GameplayStatics.SaveGameToSlot` _returnvalue_3 "GlobalOptions")
      (return (`/Game/Blueprints/SaveGame/GlobalOptionsSaveGame.GlobalOptions` _returnvalue_3)))))

(fn `SetGlobalOptions`
  (params (NewOptions :type "/Game/Blueprints/SaveGame/GlobalOptionsStruct Structure") (Instant :type Boolean))
  (locals (NewGlobalOptions :type "/Game/Blueprints/SaveGame/GlobalOptionsStruct Structure"))
  (bind _output_get (set `local.NewGlobalOptions` NewOptions))
  (bind _returnvalue (select `bool` (`.bSoundFX_5_56B5C2924CF9C7E9F7B560884393B480` (break `/Game/Blueprints/SaveGame/GlobalOptionsStruct` _output_get)) :`true` 1.0))
  (`GameplayStatics.SetSoundMixClassOverride` "/Game/Assets/AudioClasses/SM_Mixer.SM_Mixer" "/Game/Assets/AudioClasses/SC_Music.SC_Music" (select `bool` (break `/Game/Blueprints/SaveGame/GlobalOptionsStruct` _output_get) :`false` 0.001 :`true` 1.0) 1.0 _returnvalue)
  (`GameplayStatics.SetSoundMixClassOverride` "/Game/Assets/AudioClasses/SM_Mixer.SM_Mixer" "/Game/Assets/AudioClasses/SC_SFX.SC_SFX" _returnvalue 1.0 (select `bool` Instant :`false` 1.0))
  (bind _returnvalue_2 (`GameplayStatics.CreateSaveGameObject` "/Game/Blueprints/SaveGame/GlobalOptionsSaveGame.GlobalOptionsSaveGame_C"))
  (set `/Game/Blueprints/SaveGame/GlobalOptionsSaveGame.GlobalOptions` (`local.NewGlobalOptions`) _returnvalue_2)
  (`GameplayStatics.SaveGameToSlot` _returnvalue_2 "GlobalOptions"))